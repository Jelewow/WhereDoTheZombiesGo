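; Base weapon actor for AI characters that fires through an EBBarrel component and activates a muzzle flash on each shot.
; StartShoot and StopShoot toggle barrel firing, with StopShoot also resetting the barrel to the muzzle flash transform.
; While shooting, Tick moves the barrel to where the owner's Weapon forward line crosses the muzzle plane, matching that component's rotation.
; DebugDraw runs each tick, but its drawing code is disconnected.
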(event `self.ReceiveBeginPlay`
  (add `EBBarrel.ShotFired` (`self.EBBarrel`) (delegate `OnShot`)))

(event `OnShot`
  (`ActorComponent.Activate` (`self.MuzzleFlash`) true))

(event `Start Shoot`
  (set `self.bIsShooting` true)
  (`self.Update Barrel Location`)
  (`EBBarrel.Shoot` (`self.EBBarrel`) true))

(event `Stop Shoot`
  (set `self.bIsShooting` false)
  (`EBBarrel.Shoot` (`self.EBBarrel`) false)
  (`SceneComponent.K2_SetWorldTransform` (`self.EBBarrel`) (`SceneComponent.K2_GetComponentToWorld` (`self.MuzzleFlash`)) false false))

(event `self.ReceiveTick`
  (params (DeltaSeconds :type "Float (single-precision)"))
  (`self.Debug Draw`)
  (if (`self.bIsShooting`)
    (`self.Update Barrel Location`)))

(fn `Debug Draw`)

(fn `Update Barrel Location`
  (bind _muzzlelocation (`self.MuzzleLocation`))
  (bind _weapon (`/Game/Zombie_Project/AI/BaseEnemy/AI_Soldier.Weapon` (`self.WeaponOwner`)))
  (bind _returnvalue (`SceneComponent.K2_GetComponentLocation` _weapon))
  (`SceneComponent.K2_SetWorldLocation` (`self.EBBarrel`) (`.Intersection` (`KismetMathLibrary.LinePlaneIntersection_OriginNormal` _returnvalue (+ _returnvalue (* (`SceneComponent.GetForwardVector` _weapon) 1000.0)) (`SceneComponent.K2_GetComponentLocation` _muzzlelocation) (`SceneComponent.GetForwardVector` _muzzlelocation))) false false)
  (`SceneComponent.K2_SetWorldRotation` (`self.EBBarrel`) (`SceneComponent.K2_GetComponentRotation` (`/Game/Zombie_Project/AI/BaseEnemy/AI_Soldier.Weapon` (`self.WeaponOwner`))) false false))

(fn `UserConstructionScript`)